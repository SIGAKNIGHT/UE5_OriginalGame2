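; MyGameInstance is the game instance that holds the player's RPG stats, level, name, game timer and stage name.
; Its Initialize function resets each of these variables to the value in the MyGameInstance class defaults, restoring a fresh state without hard-coded values.
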(fn Initialize
  (bind (_vitality _concentration _endurance _strength _dexterity _resistance _intelligence _bloodtinge _level _gametimer _stagename _playername) (Utilities|GetClassDefaults "MyGameInstance_C"))
  (Variables|Default|SetVitality _vitality)
  (Variables|Default|SetConcentration _concentration)
  (Variables|Default|SetEndurance _endurance)
  (Variables|Default|SetStrength _strength)
  (Variables|Default|SetDexterity _dexterity)
  (Variables|Default|SetResistance _resistance)
  (Variables|Default|SetIntelligence _intelligence)
  (Variables|Default|SetBloodtinge _bloodtinge)
  (Variables|Default|SetLevel _level)
  (Variables|Default|SetGameTimer _gametimer)
  (Variables|Default|SetStageName _stagename)
  (Variables|Default|SetPlayerName _playername))