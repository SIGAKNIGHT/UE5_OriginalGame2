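; BP_AIPaladin_UE1 is a Paladin boss enemy that slashes when the player comes close and drives an on-screen boss HP bar.
; BeginPlay creates the HP widget and sets the boss name.
; Tick measures distance to the player and plays the slash montage within range, gated by falling, motion-lock and attacking checks that clear when the montage ends.
; Tick also pushes health ratios and total damage to the widget, with debug prints.
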(event Collision|EventActorBeginOverlap
  (params (OtherActor :type Actor%20Object%20Reference)))

(event EventTick
  (params (DeltaSeconds :type Float%20%28single-precision%29))
  (bind _bp_hp (Variables|Default|GetBP_HP))
  (bind _bp_hp_2 (Variables|Default|GetBP_HP))
  (bind _bp_hp_3 (Variables|Default|GetBP_HP))
  (bind _bp_hp_4 (Variables|Default|GetBP_HP))
  (bind _totaldamage (Variables|/Game/Blueprints/Player/BP_HP.BP_HP_C|GetTotalDamage _bp_hp_3))
  (Utilities|FlowControl|Sequence
    (:then_0
      (bind _output_get (Variables|Default|SetDistance (Math|Vector|VectorLength (- (Transformation|GetWorldLocation (Variables|Character|GetMesh)) (Transformation|GetWorldLocation (Variables|/Script/Engine.Character|GetMesh (Game|GetPlayerCharacter 0)))))))
      (Development|PrintString (Class|KismetStringLibrary|BuildStringDouble "Distance " "" _output_get) true true "(R=1.000000,G=0.000000,B=1.000000,A=1.000000)" 0.0))
    (:then_1
      (if (not (Variables|Default|GetIs%20Attacking))
        (if (<= (Variables|Default|GetDistance) 2e+02)
          ;[1 1 1] R1攻撃
          (Utilities|CheckFallingandMotionLock
            (:OK
              (if (not (Variables|Default|GetIs%20Attacking)) ; 攻撃中でないなら
                (Variables|Default|SetMotionLock true)
                (Variables|Default|SetIs%20Attacking true)
                (Animation|Montage|PlayMontage (Variables|Character|GetMesh) "/Game/AnimMontage/Paladin_UE5/slash_UE_Montage.slash_UE_Montage"
                  (:then
                    (Development|PrintString "Attack" true true "(R=1.000000,G=0.000000,B=0.000000,A=1.000000)"))
                  (:OnCompleted
                    (Variables|Default|SetIs%20Attacking false :!label _label) ; 攻撃が終了、中断されたらフラグオフ
                    (Variables|Default|SetMotionLock false))
                  (:OnInterrupted
                    (goto _label)))))))))
    (:then_2
      (Utilities|FlowControl|Sequence
        (:then_1
          ;[1 1 1] コメント
          (Variables|/Game/MaedaDaiki/Blueprints/BossHP_WBP.BossHP_WBP_C|SetWBP_HP (Variables|Default|GetBossHP_Widget) (/ (Variables|/Game/Blueprints/Player/BP_HP.BP_HP_C|GetHP _bp_hp) (Variables|/Game/Blueprints/Player/BP_HP.BP_HP_C|GetMaxHP _bp_hp)))
          (Variables|/Game/MaedaDaiki/Blueprints/BossHP_WBP.BossHP_WBP_C|SetWBP_LastHP (Variables|Default|GetBossHP_Widget) (/ (Variables|/Game/Blueprints/Player/BP_HP.BP_HP_C|GetLastHP _bp_hp_2) (Variables|/Game/Blueprints/Player/BP_HP.BP_HP_C|GetMaxHP _bp_hp_2)))
          (Development|PrintString (Utilities|StatusPrintString "BossHP" (Variables|/Game/Blueprints/Player/BP_HP.BP_HP_C|GetHP _bp_hp_4) (Variables|/Game/Blueprints/Player/BP_HP.BP_HP_C|GetMaxHP _bp_hp_4)) true false "(R=0.600000,G=0.000000,B=0.000000,A=1.000000)" 0.0)
          (Variables|/Game/MaedaDaiki/Blueprints/BossHP_WBP.BossHP_WBP_C|SetWBP_BossDamage (Variables|Default|GetBossHP_Widget) (Math|Float|Truncate _totaldamage))
          (Development|PrintString (Utilities|String|ToString(Float) _totaldamage) true false "(R=0.600000,G=0.000000,B=0.000000,A=1.000000)" 0.0))))))

(event EventBeginPlay
  (Utilities|FlowControl|Sequence
    (:then_0
      ;[1 1 1] HPゲージ作成
      (bind _returnvalue (UserInterface|CreateWidget "/Game/MaedaDaiki/Blueprints/BossHP_WBP.BossHP_WBP_C"))
      (bind _output_get (Variables|Default|SetBossHP_Widget _returnvalue))
      (Widget|SetVisibility _output_get "Visible")
      (UserInterface|Viewport|AddtoViewport _output_get 0))
    (:then_1
      ;[1 1 1] 名前設定
      (bind _output_get_2 (Variables|Default|SetEnemyName "ぼすーーーーー"))
      (Default|DispSetEnemyNameEvent (Variables|Default|GetBossHP_Widget) _output_get_2))))

(fn ConstructionScript
  (|CallParentFunction))