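; Component that removes a boss wall by fading it out and destroying the target actor.
; EndBossWall takes the first child of TargetActor's root as a mesh and gives it a dynamic instance of a boss wall material.
; A timeline drives Opacity from the inverse of its value, then hides the mesh and destroys the actor on finish.
; A test timer in Tick and debug prints remain.
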(event Custom|EndBossWall
  (bind _targetactor (Variables|Default|GetTargetActor))
  (bind _asmesh_component (Utilities|Casting|CastToMeshComponent (Components|GetChildComponent (Variables|/Script/Engine.Actor|GetRootComponent _targetactor) 0))
    (:then
      (Rendering|Material|CreateDynamicMaterialInstance _asmesh_component 0 "/Game/MaedaDaiki/Material/MT_BossWall_Copy.MT_BossWall_Copy" "None" :!class /Script/Engine.PrimitiveComponent)
      (bind _alpha (Utilities|TimeLine 1.5)
        (:Update
          (Development|PrintString (Utilities|String|ToString(Float) (- 1.0 _alpha)))
          (Rendering|Material|SetScalarParameterValueonMaterials _asmesh_component "Opacity" (- 1.0 _alpha)))
        (:Finish
          (Rendering|SetVisibility _asmesh_component false false)
          (Actor|DestroyActor _targetactor))))
    (:CastFailed
      (Development|PrintString "Hello"))))

(event EventBeginPlay)

(event EventTick
  (params (DeltaSeconds :type Float%20%28single-precision%29))
  ;[1 1 1] テスト用
  (Variables|Default|Settimer (+ DeltaSeconds (Variables|Default|Gettimer)))
  (if (>= (Variables|Default|Gettimer) 1e+01)
    (Variables|Default|Settimer -1e+02)))