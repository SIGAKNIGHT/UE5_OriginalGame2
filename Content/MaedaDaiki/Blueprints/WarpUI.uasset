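; WarpUI shows the warp icon and opens the warp menu when the player is near a Warp_Point.
; Each Tick, it checks Sphere2 for overlapping Warp_Point actors and tells HUD_Warp to show or hide the icon.
; IA_Select repeats the overlap check to open the menu, only if it is not already shown and the HUD's hidden timer has run out, preventing an immediate reopen.
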(event Input|EnhancedActionEvents|EnhancedInputActionIA_Select
  (params (ActionValue :type Boolean) (ElapsedSeconds :type Float%20%28double-precision%29) (TriggeredSeconds :type Float%20%28double-precision%29) (InputAction :type Input%20Action%20Object%20Reference :default "/Game/Input/IA_Select.IA_Select"))
  ;[1 1 1] Eキーを押したときにプレイヤーの前方にワープオブジェクトがあったらワープメニューを表示
  (:Triggered
    (bind _ashud_warp (Utilities|Casting|CastToHUD_Warp (HUD|GetHUD (Game|GetPlayerController 0)))) ; 出て入るのを阻止するため
    (if (<= (Variables|/Game/MaedaDaiki/Blueprints/HUD_Warp.HUD_Warp_C|GetWarpMenuHiddenTimer _ashud_warp) 0.0)
      (if (not (Variables|/Game/MaedaDaiki/Blueprints/HUD_Warp.HUD_Warp_C|GetIsShowWarpMenu _ashud_warp)) ; ワープメニューが表示じょうたいでない
        ;;[1 1 1] ループで当たっているかを調べる
        (Utilities|Array|ForEachLoopwithBreak (Collision|GetOverlappingActors (Variables|Default|GetSphere2) "/Game/MaedaDaiki/Blueprints/Warp_Point.Warp_Point_C" :!class /Script/Engine.PrimitiveComponent) :!label _label
          (:LoopBody
            (bind _ashud_warp_2 (Utilities|Casting|CastToHUD_Warp (HUD|GetHUD (Game|GetPlayerController 0))))
            (Default|DispWarpMenuEvent _ashud_warp_2 true)
            (goto _label Break)))))))

(event EventBeginPlay)

(event EventTick
  (params (DeltaSeconds :type Float%20%28single-precision%29))
  ;[1 1 1] ワープIcon表示非表示
  (CallFunction|WarpIconVSPlayer DeltaSeconds :!pinned true) ; ワープアイコン表示/非表示
)

(fn WarpIconVSPlayer
  (params (DeltaTime :type Float%20%28double-precision%29))
  (bind _returnvalue (Game|GetPlayerController 0))
  (bind _returnvalue_2 (HUD|GetHUD _returnvalue))
  (Utilities|Array|ForEachLoopwithBreak (Collision|GetOverlappingActors (Variables|Default|GetSphere2) "/Game/MaedaDaiki/Blueprints/Warp_Point.Warp_Point_C" :!class /Script/Engine.PrimitiveComponent)
    (:LoopBody
      (bind _ashud_warp (Utilities|Casting|CastToHUD_Warp _returnvalue_2 :!pinned true)) ; 当たっていたら
      (Default|DispWarpiconEvent _ashud_warp true :!pinned true) ; Icon表示
      (return))
    (:Completed
      (bind _ashud_warp_2 (Utilities|Casting|CastToHUD_Warp _returnvalue_2 :!pinned true)) ; 当たっていなかった
      (Default|DispWarpiconEvent _ashud_warp_2 false :!pinned true) ; Icon非表示
      (return))))