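; Child enemy Blueprint for the "Taurus Demon" boss-style character, handling its battle intro, attacks and death.
; BattleStart starts an EnemyEnum state machine run from Tick: walk forward, roar, then idle, with IsFirstAction set as the roar blends out.
; AttackR1 and AttackR2 play the same swipe montage behind re-entry guards.
; Death passes a montage to the parent, then spawns delayed Niagara particles; a material fade-out sits unwired.
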(event EventBeginPlay
  (Variables|Default|SetEnemyName "Taurus Demon")
  (|CallParentFunction))

(event Collision|EventActorBeginOverlap
  (params (OtherActor :type Actor%20Object%20Reference))
  (|CallParentFunction OtherActor) ; このノードは無効になっているため呼び出せません。\n機能をビルドするにはピンをドラッグしてください。
)

(event EventTick
  (params (DeltaSeconds :type Float%20%28single-precision%29))
  ;[1 1 1] Tick
  (|CallParentFunction DeltaSeconds)
  (switch Utilities|FlowControl|Switch|SwitchonEnemyEnum (Variables|Default|GetEnemyEnum)
    (:NewEnumerator1
      (CallFunction|WalkForward))
    (:NewEnumerator2
      (CallFunction|Roar))))

(event EventActive
  (|CallParentFunction))

(event Custom|Roar
  (if (not (CallFunction|IsFalling))
    (Utilities|FlowControl|Delay 1.5)
    (Utilities|FlowControl|DoOnce false :!label _label
      (:Completed
        (Animation|Montage|PlayMontage (Variables|Character|GetMesh) "/Game/AnimMontage/MawJLaygo/mutantroaring_UE_Montage.mutantroaring_UE_Montage" 1.5
          (:OnCompleted
            (Variables|Default|SetEnemyEnum "NewEnumerator3")
            (goto _label Reset))
          (:OnBlendOut
            (Variables|Default|SetIsFirstAction true)))))))

(event Custom|WalkForward
  (CallFunction|Move 0.0 0.5)
  (Utilities|FlowControl|DoOnce false
    (:Completed
      (Utilities|FlowControl|Delay 0.5)
      (Variables|Default|SetEnemyEnum "NewEnumerator2"))))

(event EventAttackR1
  (Utilities|FlowControl|DoOnce false :!label _label
    (:Completed
      (Animation|Montage|PlayMontage (Variables|Character|GetMesh) "/Game/AnimMontage/MawJLaygo/mutantswiping_UE_Montage.mutantswiping_UE_Montage"
        (:OnCompleted
          (goto _label Reset))
        (:OnInterrupted
          (goto _label Reset))))))

(event EventDeath
  (params (MontageToPlay :type Anim%20Montage%20Object%20Reference))
  (|CallParentFunction "/Game/AnimMontage/MawJLaygo/StandingReactDeathForward_UE_Montage.StandingReactDeathForward_UE_Montage")
  (Utilities|FlowControl|Delay 3.0)
  (Utilities|FlowControl|Sequence
    (:then_0
      (Niagara|SpawnSystemAttached "/Game/MaedaDaiki/Blueprints/DeathNiagaraSystem.DeathNiagaraSystem" (Variables|Character|GetMesh) "None" "0, 0, 0" "0, 0, 0" "SnapToTarget" true :!pinned true) ; パーティクル生成
    )))

(event EventBattleStart
  (Utilities|FlowControl|DoOnce false
    (:Completed
      (Variables|Default|SetEnemyEnum "NewEnumerator1"))))

(event EventAttackR2
  (Utilities|FlowControl|DoOnce false :!label _label
    (:Completed
      (Animation|Montage|PlayMontage (Variables|Character|GetMesh) "/Game/AnimMontage/MawJLaygo/mutantswiping_UE_Montage.mutantswiping_UE_Montage"
        (:OnCompleted
          (goto _label Reset))
        (:OnInterrupted
          (goto _label Reset))))))

(fn ConstructionScript
  (|CallParentFunction))