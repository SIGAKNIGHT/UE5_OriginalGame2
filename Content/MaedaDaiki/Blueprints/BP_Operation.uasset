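; BP_Operation is a trigger actor that shows an operation message widget while the player is inside its Box volume.
; On BeginPlay it creates a WBP_Operation widget, adds it to the viewport collapsed, and passes its Int variable to SetMessage.
; Box overlap events cast to BP_Player, making the widget visible on entry and collapsing it on exit.
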(event OnComponentBeginOverlap(Box)
  (params (OverlappedComponent :type Primitive%20Component%20Object%20Reference) (OtherActor :type Actor%20Object%20Reference) (OtherComp :type Primitive%20Component%20Object%20Reference) (OtherBodyIndex :type Integer) (bFromSweep :type Boolean) (SweepResult :type Hit%20Result%20Structure%20%28by%20ref%29))
  (Utilities|Casting|CastToBP_Player OtherActor)
  (Widget|SetVisibility (Variables|Default|GetWBP_Operation) "Visible"))

(event OnComponentEndOverlap(Box)
  (params (OverlappedComponent :type Primitive%20Component%20Object%20Reference) (OtherActor :type Actor%20Object%20Reference) (OtherComp :type Primitive%20Component%20Object%20Reference) (OtherBodyIndex :type Integer))
  (Utilities|Casting|CastToBP_Player OtherActor)
  (Widget|SetVisibility (Variables|Default|GetWBP_Operation) "Collapsed"))

(event EventBeginPlay
  (bind _returnvalue (UserInterface|CreateWidget "/Game/MaedaDaiki/Blueprints/WBP_Operation.WBP_Operation_C"))
  (bind _output_get (Variables|Default|SetWBP_Operation _returnvalue))
  (Widget|SetVisibility _output_get "Collapsed")
  (UserInterface|Viewport|AddtoViewport _output_get 20)
  (Default|SetMessage (Variables|Default|GetWBP_Operation) (Variables|Default|GetInt)))

(event Collision|EventActorBeginOverlap
  (params (OtherActor :type Actor%20Object%20Reference)))

(event EventTick
  (params (DeltaSeconds :type Float%20%28single-precision%29)))

(fn ConstructionScript)