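; Background music Blueprint that starts and stops the boss fight track.
; Tick polls the player's BossWallEntry.IsInBossStage through a DoOnce that re-arms while the flag is false, so BossBGM starts only once.
; A failed cast to BP_Player leaves the DoOnce closed, ending the polling.
; EndBossBGM fades the track out over one second and has no caller in this graph.
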(event Custom|StartBossBGM
  (Audio|Components|Audio|Play (Variables|Default|GetBossBGM) 0.0))

(event Custom|EndBossBGM
  (Audio|Components|Audio|FadeOut (Variables|Default|GetBossBGM) 1.0 0.0 "Linear" :!class /Script/Engine.AudioComponent))

(event EventBeginPlay)

(event Collision|EventActorBeginOverlap
  (params (OtherActor :type Actor%20Object%20Reference)))

(event EventTick
  (params (DeltaSeconds :type Float%20%28single-precision%29))
  (Utilities|FlowControl|DoOnce false :!label _label
    (:Completed
      (bind _asbp_player (Utilities|Casting|CastToBP_Player (Game|GetPlayerCharacter 0)))
      (if (Variables|/Game/MaedaDaiki/Blueprints/BossWallEntry.BossWallEntry_C|GetIsInBossStage (Variables|/Game/Blueprints/Player/BP_Player.BP_Player_C|GetBossWallEntry _asbp_player))
        (CallFunction|StartBossBGM)
        (else
          (goto _label Reset))))))

(fn ConstructionScript)