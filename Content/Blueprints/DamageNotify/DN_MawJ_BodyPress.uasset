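; Anim notify state that opens the damage window for MawJ Laygo's body press attack.
; On begin it casts the mesh owner to BP_MawJLaygo and calls SwordActive on the BP_BaseWeapon held in its Body child actor component.
; On end it calls SwordDeactive on that same weapon, so the notify's span in the animation sets how long the body weapon is active.
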(fn ReceivedNotifyBegin
  (params (MeshComp :type Skeletal%20Mesh%20Component%20Object%20Reference) (Animation :type Anim%20Sequence%20Base%20Object%20Reference) (TotalDuration :type Float%20%28single-precision%29) (EventReference :type Anim%20Notify%20Event%20Reference%20Structure%20%28by%20ref%29))
  (bind _asbp_maw_jlaygo (Utilities|Casting|CastToBP_MawJLaygo (Components|GetOwner MeshComp)))
  (bind _asbp_base_weapon (Utilities|Casting|CastToBP_BaseWeapon (Variables|/Script/Engine.ChildActorComponent|GetChildActor (Variables|/Game/Blueprints/Enemy/BP_MawJLaygo.BP_MawJLaygo_C|GetBody _asbp_maw_jlaygo))))
  (Default|SwordActive _asbp_base_weapon)
  (return false))

(fn ReceivedNotifyEnd
  (params (MeshComp :type Skeletal%20Mesh%20Component%20Object%20Reference) (Animation :type Anim%20Sequence%20Base%20Object%20Reference) (EventReference :type Anim%20Notify%20Event%20Reference%20Structure%20%28by%20ref%29))
  (bind _asbp_maw_jlaygo (Utilities|Casting|CastToBP_MawJLaygo (Components|GetOwner MeshComp)))
  (bind _asbp_base_weapon (Utilities|Casting|CastToBP_BaseWeapon (Variables|/Script/Engine.ChildActorComponent|GetChildActor (Variables|/Game/Blueprints/Enemy/BP_MawJLaygo.BP_MawJLaygo_C|GetBody _asbp_maw_jlaygo))))
  (Default|SwordDeactive _asbp_base_weapon)
  (return false))