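; BP_Character is a character Blueprint with health, damage and death handling, apparently a base whose damage and death events are left empty.
; Tick updates speed percentage, a local-axis speed vector and the spine_03 transform, and kills the character after over three seconds of falling.
; AnyDamage subtracts multiplied damage from BPHP, calling OnDamaged, or OnDead once HP turns negative.
; Helpers cover angles, tags, launching, movement toggling, debugging and an armor-based damage formula.
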(event Custom|OnDamaged)

(event Custom|FallDead)

(event Custom|AnyDamage
  (params (Damage :type Float%20%28double-precision%29) (Multi :type Float%20%28double-precision%29))
  (bind _bp_hp (Variables|Default|GetBP_HP))
  ;[1 1 1] 被ダメージ
  (bind _output_get (Variables|/Game/Blueprints/BP_HP.BP_HP_C|SetHP _bp_hp (- (Variables|/Game/Blueprints/BP_HP.BP_HP_C|GetHP _bp_hp) (* Damage Multi))))
  (if (>= _output_get 0.0)
    (CallFunction|OnDamaged)
    (elif (Variables|Default|GetIsAlive)
      (Variables|Default|SetIsAlive false)
      (CallFunction|OnDead))))

(event Custom|OnDead
  (params (Montage%20to%20play :type Anim%20Montage%20Object%20Reference)))

(event EventBeginPlay)

(event Collision|EventActorBeginOverlap
  (params (OtherActor :type Actor%20Object%20Reference)))

(event EventTick
  (params (DeltaSeconds :type Float%20%28single-precision%29))
  (bind _charactermovement (Variables|Character|GetCharacterMovement))
  (Utilities|FlowControl|Sequence
    (:then_0
      ;[1 1 1] 移動成分の速度から速度と対地速度を設定する。
      ; 対地速度は速度のX軸とY軸のみから計算されるので、上下に動いても影響はありません。
      (bind _output_get (Variables|Default|SetVelocity (Variables|/Script/Engine.MovementComponent|GetVelocity _charactermovement)))
      (Variables|Default|SetSpeed (* (/ (Math|Vector|VectorLengthXY _output_get) (Variables|/Script/Engine.CharacterMovementComponent|GetMaxWalkSpeed _charactermovement)) 1e+02)))
    (:then_1
      ;[1 1 1] Xスピード
      (Variables|Default|SetSpeedVec (Math|Vector2D|MakeVector2D (/ (Math|Vector|DotProduct (Variables|Default|GetVelocity) (Transformation|GetActorRightVector self)) (Math|Float|Max(Float) 1.0 (Class|MovementComponent|GetMaxSpeed (Variables|Character|GetCharacterMovement)))) (/ (Math|Vector|DotProduct (Variables|Default|GetVelocity) (Transformation|GetActorForwardVector self)) (Math|Float|Max(Float) 1.0 (Class|MovementComponent|GetMaxSpeed (Variables|Character|GetCharacterMovement)))))))
    (:then_2
      (Variables|Default|SetSpine03 (CallFunction|GetSpine03)))
    (:then_3
      (if (CallFunction|IsFalling)
        (bind _output_get_2 (Variables|Default|SetFallingTimer (+ (Variables|Default|GetFallingTimer) DeltaSeconds)))
        (if (> _output_get_2 3.0)
          (Utilities|FlowControl|DoOnce false :!label _label
            (:Completed
              (Variables|/Game/Blueprints/BP_HP.BP_HP_C|SetHP (Variables|Default|GetBP_HP) 0.0)
              (Variables|Default|SetIsAlive false)
              (CallFunction|FallDead))))
        (else
          (Variables|Default|SetFallingTimer 0.0)
          (goto _label Reset))))))

(fn ConstructionScript)

(fn CalcAngle
  (params (Front :type Vector) (PtoE :type Vector))
  (return (Class|KismetMathLibrary|DegAcos (Math|Vector|DotProduct (Math|Vector|Normalize Front) (Math|Vector|Normalize PtoE)))))

(fn IsFalling
  (return (AI|Components|NavMovement|IsFalling (Variables|Character|GetCharacterMovement))))

(fn StatusPrintString
  (params (Status :type String) (Current :type Float%20%28double-precision%29) (Max :type Float%20%28double-precision%29))
  (return (Utilities|String|Append Status (Utilities|String|ToString(Float) Current) "/" (Utilities|String|ToString(Float) Max))))

(fn TagCheck
  (params (ターゲット :type Actor%20Object%20Reference) (Tag :type Name))
  (return (Actor|ActorHasTag ターゲット Tag)))

(fn FCLaunchCharacter
  (params (XY_Value :type Float%20%28double-precision%29) (Z_Value :type Float%20%28double-precision%29))
  (Character|LaunchCharacter (+ (* (Transformation|GetActorForwardVector) XY_Value) (Math|Vector|MakeVector 0.0 0.0 Z_Value)) false false))

(fn Movement
  (params (CanMove :type Boolean))
  (if CanMove
    (Pawn|Components|CharacterMovement|SetMovementMode (Variables|Character|GetCharacterMovement) "MOVE_Walking" 0)
    (else
      (Pawn|Components|CharacterMovement|DisableMovement (Variables|Character|GetCharacterMovement)))))

(fn DebugForwardVector
  (params (Mesh :type Skeletal%20Mesh%20Component%20Object%20Reference) (Actor :type Actor%20Object%20Reference))
  (bind _returnvalue (Transformation|GetActorLocation Actor))
  (Rendering|Debug|DrawDebugSphere _returnvalue 16.0 12 "(R=1.000000,G=0.000000,B=1.000000,A=1.000000)" 0.0)
  (Rendering|Debug|DrawDebugArrow _returnvalue (+ _returnvalue (* (Transformation|GetActorForwardVector Actor) 1e+02)) 1e+02 "(R=1.000000,G=0.000000,B=1.000000,A=1.000000)" 0.0 1.0))

(fn GetSpine03
  (return (Transformation|GetSocketTransform (Variables|Character|GetMesh) "spine_03" "RTS_World")))

(fn CalcRealDamage
  (params (Damage :type Float%20%28double-precision%29) (Armor :type Integer))
  (return (* Damage (* 0.9 (- 1 (Class|KismetMathLibrary|Exp (* -0.5 (/ Damage Armor))))))))