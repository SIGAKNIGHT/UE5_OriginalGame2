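; Stamina Blueprint that starts at maximum and exposes functions to consume stamina and check whether enough remains.
; Each tick it clamps values, then drains a trailing temporary stamina value down toward real stamina after a short delay, like a delayed bar drop.
; After a longer pause it regenerates stamina at a steady per-second rate.
; Comparing against last frame's stamina restarts both timers whenever more stamina is spent.
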(event EventBeginPlay
  (Variables|Default|SetStamina (Variables|Default|GetMaxStamina)))

(event EventTick
  (params (DeltaSeconds :type Float%20%28single-precision%29))
  (CallFunction|UpdateStamina DeltaSeconds))

(fn UpdateStamina
  (params (ElapsedTime :type Float%20%28double-precision%29))
  (Utilities|FlowControl|Sequence
    (:then_0
      ;[1 1 1] クランプ
      (Variables|Default|SetStamina (Math|Float|Min(Float) (Variables|Default|GetStamina) (Variables|Default|GetMaxStamina)))
      (Variables|Default|SetTemporalyStamina (Math|Float|Min(Float) (Variables|Default|GetTemporalyStamina) (Variables|Default|GetMaxStamina))))
    (:then_1
      ;[1 1 1] 仮スタミナ計算
      (Utilities|TemporalyStamina>Stamina ; スタミナ消費後なら
        (:true
          (Utilities|OldStamina>Stamina ; 追加でスタミナ消費していれば
            (:true
              (bind _output_get (Variables|Default|SetDelayTimer 0.0)))
            (:false
              _))
          (if (>= _output_get 0.1) ; 遅延タイマーが指定秒数以上なら
            (|CollapseGraph) ; 仮スタミナを徐々に減少
          )
          (Variables|Default|SetDelayTimer (+ (Variables|Default|GetDelayTimer) ElapsedTime)))
        (:false
          (Variables|Default|SetDelayTimer 0.0)
          (Variables|Default|SetTemporalyStamina (Variables|Default|GetStamina)))))
    (:then_2
      ;[1 1 1] スタミナ回復
      (Utilities|Stamina<MaxStamina ; スタミナがMaxではない
        (:true
          (Utilities|OldStamina>Stamina ; 追加でダメージを受けていたら
            (:true
              (bind _output_get_2 (Variables|Default|SetHealTimer 0.0)))
            (:false
              _))
          (if (>= _output_get_2 1.5) ; 指定秒数経過したら
            (|CollapseGraph_2) ; スタミナを徐々に回復
          )
          (Variables|Default|SetHealTimer (+ (Variables|Default|GetHealTimer) ElapsedTime)))
        (:false
          (Variables|Default|SetHealTimer 0.0))))
    (:then_3
      (Variables|Default|SetOldStamina (Variables|Default|GetStamina)))))

(fn StaminaConsumption
  (params (Value :type Float%20%28double-precision%29))
  (bind _output_get (Variables|Default|SetStamina (- (Variables|Default|GetStamina) Value))) ; スタミナを減らす
  (return _output_get))

(fn StaminaCheck
  (params (Value :type Float%20%28double-precision%29))
  (bind _output_get (LocalVariables|Setbool (>= (Variables|Default|GetStamina) Value)))
  (return _output_get))