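; BP_Item tracks the player's count of "Est" uses, apparently a limited-charge consumable, and mirrors it to the equipment UI.
; The count resets to its maximum on BeginPlay or through the ResetEst event.
; SetWBP stores the player equipment widget and writes the current count to it.
; UseEst decrements the count and updates that text directly, while EstCheck separately reports whether any uses remain.
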(event Custom|ResetEst
  (Variables|Default|SetEstNum (Variables|Default|GetMaxEstNum)))

(event EventBeginPlay
  (CallFunction|ResetEst))

(event EventTick
  (params (DeltaSeconds :type Float%20%28single-precision%29)))

(fn SetWBP
  (params (WBP :type WBP%20Player%20Equipment%20Object%20Reference))
  (Variables|Default|SetWBP_PlayerEquipment WBP)
  (Variables|/Game/MaedaDaiki/Blueprints/WBP_PlayerEquipment.WBP_PlayerEquipment_C|SetEstNum2 (Variables|Default|GetWBP_PlayerEquipment) (Utilities|Text|ToText(Integer) (Variables|Default|GetEstNum))))

(fn UseEst
  (bind _result (Math|Integer|DecrementInt (Variables|Default|GetEstNum))
    (:%20%20
      (Variables|/Game/MaedaDaiki/Blueprints/WBP_PlayerEquipment.WBP_PlayerEquipment_C|SetEstNum2 (Variables|Default|GetWBP_PlayerEquipment) (Utilities|Text|ToText(Integer) _result))
      (return))))

(fn EstCheck
  (return (> (Variables|Default|GetEstNum) 0)))