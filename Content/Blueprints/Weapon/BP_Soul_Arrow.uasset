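; BP_Soul_Arrow is a soul arrow projectile that damages characters it hits.
; ResetTarget launches it by setting the ProjectileMovement velocity in local space from the supplied vector.
; On Hit, it ignores its owner, otherwise destroys itself and applies Damage to a BP_Character, printing a debug string for anything else.
; Impact emitter and sound spawns exist but are unconnected, so they never run.
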(event Custom|ResetTarget
  (params (vector :type Vector))
  (Game|Components|ProjectileMovement|SetVelocityinLocalSpace (Variables|Default|GetProjectileMovement) vector) ; ソウルの矢を指定した方向に指定した速度で飛ばす
)

(event EventBeginPlay)

(event Collision|EventActorBeginOverlap
  (params (OtherActor :type Actor%20Object%20Reference)))

(event EventTick
  (params (DeltaSeconds :type Float%20%28single-precision%29)))

(event Collision|EventHit
  (params (MyComp :type Primitive%20Component%20Object%20Reference) (Other :type Actor%20Object%20Reference) (OtherComp :type Primitive%20Component%20Object%20Reference) (bSelfMoved :type Boolean) (HitLocation :type Vector :default "0, 0, 0") (HitNormal :type Vector :default "0, 0, 0") (NormalImpulse :type Vector :default "0, 0, 0") (Hit :type Hit%20Result%20Structure%20%28by%20ref%29))
  (if (!= Other (Components|GetOwner))
    (Actor|DestroyActor)
    (Utilities|Casting|CastToBP_Character Other
      (:then
        (Game|Damage|ApplyDamage Other (Variables|Default|GetDamage) 0 0))
      (:CastFailed
        (Development|PrintString "N")))))

(fn ConstructionScript)