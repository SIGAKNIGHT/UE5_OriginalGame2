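; BP_BaseAmmo is a weapon projectile, apparently the base ammo class, that damages characters it overlaps.
; On overlap it ignores its owner and anything other than a BP_Character, then destroys itself and applies its Damage value.
; ResetTarget launches it by setting the ProjectileMovement velocity in local space.
; Impact emitter and sound nodes exist but are unconnected, and the Hit event is empty.
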(event Custom|ResetTarget
  (params (vector :type Vector))
  (Game|Components|ProjectileMovement|SetVelocityinLocalSpace (Variables|Default|GetProjectileMovement) vector) ; 弾を指定した方向に指定した速度で飛ばす
)

(event EventBeginPlay)

(event EventTick
  (params (DeltaSeconds :type Float%20%28single-precision%29)))

(event Collision|EventHit
  (params (MyComp :type Primitive%20Component%20Object%20Reference) (Other :type Actor%20Object%20Reference) (OtherComp :type Primitive%20Component%20Object%20Reference) (bSelfMoved :type Boolean) (HitLocation :type Vector :default "0, 0, 0") (HitNormal :type Vector :default "0, 0, 0") (NormalImpulse :type Vector :default "0, 0, 0") (Hit :type Hit%20Result%20Structure%20%28by%20ref%29)))

(event Collision|EventActorBeginOverlap
  (params (OtherActor :type Actor%20Object%20Reference))
  (if (!= OtherActor (Components|GetOwner))
    (Utilities|Casting|CastToBP_Character OtherActor)
    (Actor|DestroyActor)
    (Game|Damage|ApplyDamage OtherActor (Variables|Default|GetDamage) 0 0)))

(fn ConstructionScript)