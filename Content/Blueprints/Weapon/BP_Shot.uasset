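; Weapon Blueprint that charges and fires a BP_Soul_Arrow magic projectile for its owner.
; Spawn creates the arrow just ahead of the mesh's head socket, and Tick keeps it there until release.
; Shot releases it along a fixed forward vector, while LockShot passes ResetTarget a scaled direction to the target in owner-local space.
; ResetDamage sets the arrow's damage from its base value through BPBattle's MajicDamage.
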(event Custom|Spawn
  (params (Mesh :type Skeletal%20Mesh%20Component%20Object%20Reference))
  ;[1 1 1] チャージ
  (bind _output_get (Variables|Default|SetMesh Mesh))
  (bind _transform (CallFunction|StartingPosition (Components|GetOwner) _output_get))
  (bind _returnvalue (Game|SpawnActorfromClass "/Game/Blueprints/Weapon/BP_Soul_Arrow.BP_Soul_Arrow_C" _transform "Undefined" "MultiplyWithRoot" (Components|GetOwner) 0))
  (Variables|Default|SetSoulArrow _returnvalue)
  (Variables|Default|SetTracking true))

(event Custom|LockShot
  (params (Target :type Vector))
  (bind _returnvalue (Components|GetOwner))
  (bind _start (Variables|Default|GetStart))
  (bind _returnvalue_2 (Transformation|GetActorTransform _returnvalue))
  (bind _returnvalue_3 (Math|Transform|InverseTransformLocation _returnvalue_2 Target))
  (bind _returnvalue_4 (Math|Transform|InverseTransformLocation _returnvalue_2 _start))
  (bind _returnvalue_5 (- _returnvalue_3 _returnvalue_4))
  (bind _returnvalue_6 (Math|Vector|Normalize _returnvalue_5))
  (bind _returnvalue_7 (* _returnvalue_6 1e+03))
  ;[1 1 1] 射撃
  (Variables|Default|SetTracking false)
  (Development|PrintString (Utilities|String|ToString(Vector) _returnvalue_7))
  (Default|ResetTarget (Variables|Default|GetSoulArrow) _returnvalue_7) ; LockOn
)

(event Custom|Shot
  ;[1 1 1] 射撃
  (Variables|Default|SetTracking false)
  (Default|ResetTarget (Variables|Default|GetSoulArrow) "1000.000000,0.000000,0.000000") ; Not LockOn
)

(event EventBeginPlay)

(event EventTick
  (params (DeltaSeconds :type Float%20%28single-precision%29))
  (if (Variables|Default|GetTracking)
    (bind _transform (CallFunction|StartingPosition (Components|GetOwner) (Variables|Default|GetMesh)))
    (Transformation|SetActorLocation (Variables|Default|GetSoulArrow) (.location _transform) false false)))

(fn StartingPosition
  (params (Actor :type Actor%20Object%20Reference) (Mesh :type Skeletal%20Mesh%20Component%20Object%20Reference))
  (bind _returnvalue (Transformation|GetActorForwardVector Actor))
  (bind _returnvalue_2 (Transformation|GetSocketTransform Mesh "head" "RTS_World"))
  (bind _returnvalue_3 (+ 34.0 16.0 5.0))
  (bind _location (Math|Transform|BreakTransform _returnvalue_2))
  (bind _returnvalue_4 (* _returnvalue _returnvalue_3))
  (bind _returnvalue_5 (+ _location _returnvalue_4))
  (Variables|Default|SetStart _returnvalue_5)
  (return (Math|Transform|MakeTransform _returnvalue_5 (Math|Rotator|MakeRotator 0.0 0.0 (.yaw (.rotation (Transformation|GetActorTransform Actor))))) "0, 0, 0"))

(fn ResetDamage
  (params (BP_Battle :type BP%20Battle%20Object%20Reference) (SoulArrow :type BP%20Soul%20Arrow%20Object%20Reference))
  (bind _damage (Default|MajicDamage BP_Battle (Variables|/Game/Blueprints/Weapon/BP_Soul_Arrow.BP_Soul_Arrow_C|GetBaseDamage SoulArrow)))
  (Variables|/Game/Blueprints/Weapon/BP_Soul_Arrow.BP_Soul_Arrow_C|SetDamage SoulArrow (Math|Conversions|ToFloat(Integer) _damage)))