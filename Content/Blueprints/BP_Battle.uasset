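; BP_Battle is a component that calculates sword damage, magic damage and armor from character stats.
; SwordDamage converts S–E scaling grades to multipliers via STRDEX, then adds Strength, Dexterity, Intelligence and Bloodtinge bonuses that grow linearly with each stat.
; SetSwordDamage writes that result to a BP_SM_Sword child actor using fixed Strength and Dexterity grades.
; MajicDamage scales base damage by Intelligence, and CalcArmor adds a Resistance bonus to BaseArmor.
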(event EventBeginPlay
  (Variables|Default|SetOwner (Components|GetOwner)))

(event EventTick
  (params (DeltaSeconds :type Float%20%28single-precision%29)))

(fn SwordDamage
  (params (WeaponDamage :type Integer) (STR :type String) (DEX :type String) (int :type String) (BLD :type String))
  (Utilities|FlowControl|Sequence
    (:then_0
      (bind _temp (Utilities|STRDEX STR))
      (LocalVariables|SetStrengthCorrection _temp))
    (:then_1
      (bind _temp_2 (Utilities|STRDEX DEX))
      (LocalVariables|SetDexterityCorrection _temp_2))
    (:then_2
      (bind _temp_3 (Utilities|STRDEX int))
      (LocalVariables|SetIntelligenceCorrection _temp_3))
    (:then_3
      (bind _temp_4 (Utilities|STRDEX BLD))
      (LocalVariables|SetBloodtingeCorrection _temp_4))
    (:then_4
      (return (+ WeaponDamage (Math|Float|Truncate (* WeaponDamage (LocalVariables|GetStrengthCorrection) (+ (* (/ (- 1.0 0.25) 98) (- (Variables|Default|GetStrength) 1)) 0.25))) (Math|Float|Truncate (* WeaponDamage (LocalVariables|GetDexterityCorrection) (+ (* (/ (- 1.0 0.25) 98) (- (Variables|Default|GetDexterity) 1)) 0.25))) (Math|Float|Truncate (* WeaponDamage (LocalVariables|GetIntelligenceCorrection) (+ (* (/ (- 1.0 0.25) 98) (- (Variables|Default|GetIntelligence) 1)) 1.0))) (Math|Float|Truncate (* WeaponDamage (LocalVariables|GetBloodtingeCorrection) (+ (* (/ (- 1.0 0.25) 98) (- (Variables|Default|GetBloodtinge) 1)) 1.0))))))))

(fn MajicDamage
  (params (BaseDamage :type Integer))
  (return (Math|Float|Truncate (* BaseDamage (/ (+ (* (/ (- 2.5e+02 1e+02) 98) (- (Variables|Default|GetIntelligence) 1)) 1e+02) 1e+02)))))

(fn SetSwordDamage
  (params (ChildActor :type Actor%20Object%20Reference))
  (bind _asbp_sm_sword (Utilities|Casting|CastToBP_SM_Sword ChildActor))
  (bind _returnvalue (CallFunction|SwordDamage (Variables|/Game/Blueprints/Weapon/BP_BaseWeapon.BP_BaseWeapon_C|GetBaseDamage _asbp_sm_sword) "C" "D"))
  (Variables|/Game/Blueprints/Weapon/BP_BaseWeapon.BP_BaseWeapon_C|SetDamage _asbp_sm_sword (Math|Conversions|ToFloat(Integer) _returnvalue)))

(fn CalcArmor
  (Variables|Default|SetArmor (+ (Variables|Default|GetBaseArmor) (+ (* 3 (- (Variables|Default|GetResistance) 1)) 1))))