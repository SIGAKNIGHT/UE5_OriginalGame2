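; BP_AutoAttack gives an owning BP_Enemy0 an automatic attack when the player comes close.
; Init stores the owner's mesh and movement component, though only the mesh is used.
; Every tick it measures the distance to player 0's mesh, prints it for debugging, and calls the owner's AttackR1 within a fixed range, with no cooldown here.
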(event Custom|Init
  (params (Mesh :type Skeletal%20Mesh%20Component%20Object%20Reference) (Character%20Movement :type Character%20Movement%20Component%20Object%20Reference))
  (Variables|Default|SetMesh Mesh)
  (Variables|Default|SetCharacterMovement Character%20Movement))

(event EventBeginPlay)

(event EventTick
  (params (DeltaSeconds :type Float%20%28single-precision%29))
  (Utilities|FlowControl|Sequence
    (:then_0
      (bind _output_get (Variables|Default|SetDistance (Math|Vector|VectorLength (- (Transformation|GetWorldLocation (Variables|Default|GetMesh)) (Transformation|GetWorldLocation (Variables|/Script/Engine.Character|GetMesh (Game|GetPlayerCharacter 0)))))))
      (Development|PrintString (Class|KismetStringLibrary|BuildStringDouble "Distance " "" _output_get) true true "(R=1.000000,G=0.000000,B=1.000000,A=1.000000)" 0.0))
    (:then_1
      (if (<= (Variables|Default|GetDistance) 2e+02)
        (bind _asbp_enemy_0 (Utilities|Casting|CastToBP_Enemy0 (Components|GetOwner)))
        (Default|AttackR1 _asbp_enemy_0)))))