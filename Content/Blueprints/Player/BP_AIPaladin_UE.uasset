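; BP_AIPaladin_UE is an AI Paladin character that automatically performs a slash attack when the player comes close.
; Each Tick it measures and debug-prints the distance between its mesh and the player's, then attacks within a fixed range if not already attacking.
; A CheckFallingAndMotionLock macro blocks attacks while falling or motion-locked.
; Attack and lock flags are set when the slash montage starts and cleared on completion or interruption.
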(event EventBeginPlay
  (|CallParentFunction) ; このノードは無効になっているため呼び出せません。\n機能をビルドするにはピンをドラッグしてください。
)

(event Collision|EventActorBeginOverlap
  (params (OtherActor :type Actor%20Object%20Reference)))

(event EventTick
  (params (DeltaSeconds :type Float%20%28single-precision%29))
  (Utilities|FlowControl|Sequence
    (:then_0
      (bind _output_get (Variables|Default|SetDistance (Math|Vector|VectorLength (- (Transformation|GetWorldLocation (Variables|Character|GetMesh)) (Transformation|GetWorldLocation (Variables|/Script/Engine.Character|GetMesh (Game|GetPlayerCharacter 0)))))))
      (Development|PrintString (Class|KismetStringLibrary|BuildStringDouble "Distance " "" _output_get) true true "(R=1.000000,G=0.000000,B=1.000000,A=1.000000)" 0.0))
    (:then_1
      (if (not (Variables|Default|GetIs%20Attacking))
        (if (<= (Variables|Default|GetDistance) 2e+02)
          ;[1 1 1] R1攻撃
          (Utilities|CheckFallingandMotionLock
            (:OK
              (if (not (Variables|Default|GetIs%20Attacking)) ; 攻撃中でないなら
                (Variables|Default|SetMotionLock true)
                (Variables|Default|SetIs%20Attacking true)
                (Animation|Montage|PlayMontage (Variables|Character|GetMesh) "/Game/AnimMontage/Paladin_UE5/slash_UE_Montage.slash_UE_Montage"
                  (:then
                    (Development|PrintString "Attack" true true "(R=1.000000,G=0.000000,B=0.000000,A=1.000000)"))
                  (:OnCompleted
                    (Variables|Default|SetIs%20Attacking false :!label _label) ; 攻撃が終了、中断されたらフラグオフ
                    (Variables|Default|SetMotionLock false))
                  (:OnInterrupted
                    (goto _label)))))))))))

(fn ConstructionScript
  (|CallParentFunction))